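; BP_ShootableActor is an actor that reacts physically to being shot or caught in an explosion.
; Point damage from bullets applies an impulse to its mesh at the hit location, opposite ShotFromDirection and scaled by damage.
; Radial damage from grenades applies a damage-scaled radial impulse from the blast origin with constant falloff.
; Any damage also prints a debug message with the amount; no health is tracked.
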(event Game|Damage|EventAnyDamage
  (params (Damage :type Float%20%28single-precision%29) (DamageType :type Damage%20Type%20Object%20Reference) (InstigatedBy :type Controller%20Object%20Reference) (DamageCauser :type Actor%20Object%20Reference))
  (Development|PrintString (Utilities|String|Append "You've Got Damage! " (Utilities|String|ToString(Float) Damage))))

(event Game|Damage|EventPointDamage
  (params (Damage :type Float%20%28single-precision%29) (DamageType :type Damage%20Type%20Object%20Reference) (HitLocation :type Vector :default "0, 0, 0") (HitNormal :type Vector :default "0, 0, 0") (HitComponent :type Primitive%20Component%20Object%20Reference) (BoneName :type Name :default "None") (ShotFromDirection :type Vector :default "0, 0, 0") (InstigatedBy :type Controller%20Object%20Reference) (DamageCauser :type Actor%20Object%20Reference) (HitInfo :type Hit%20Result%20Structure%20%28by%20ref%29))
  ;[1 1 1] Manage Damage Reaction for Bullets
  (Physics|AddImpulseatLocation (Variables|Default|GetMesh) (* ShotFromDirection (* Damage -1.0 8e+02)) HitLocation "None"))

(event Game|Damage|EventRadialDamage
  (params (DamageReceived :type Float%20%28single-precision%29) (DamageType :type Damage%20Type%20Object%20Reference) (Origin :type Vector :default "0, 0, 0") (HitInfo :type Hit%20Result%20Structure%20%28by%20ref%29) (InstigatedBy :type Controller%20Object%20Reference) (DamageCauser :type Actor%20Object%20Reference))
  ;[1 1 1] Manage Damage Reaction for Grenades
  (Physics|AddRadialImpulse (Variables|Default|GetMesh) Origin 3e+02 (* DamageReceived 6e+02) "RIF_Constant" false))

(fn ConstructionScript)