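; Grenade launcher weapon, a child of a base weapon, that fires BP_ProjectTile_Grenade projectiles from its muzzle arrow.
; StartFire passes a DoOnce gate that resets after a FireTime delay, limiting fire rate, and triggers montage, sound, muzzle flash and camera shake.
; StopFire shuts those effects off, though it stops the rifle fire montage rather than the launcher's.
; The construction script sets the weapon type and launcher-specific effect assets.
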(event Custom|Stopfx
  (bind _owningcharacter (Variables|Default|GetOwningCharacter))
  ;[1 1 1] Stop Fire Animation Montage
  (Utilities|IsValid _owningcharacter
    (:Is%20Valid
      (Animation|Montage|MontageStop (Components|SkeletalMesh|GetAnimInstance (Variables|/Game/UE_FPS/Core/BP_ShooterCharacter.BP_ShooterCharacter_C|GetMesh1P _owningcharacter)) 0.1 "/Game/Animations/FPP_Animations/HerroFPP_RifleFire_Montage.HerroFPP_RifleFire_Montage"))
    (:Is%20Not%20Valid
      _))
  ;[1 1 1] Stop Sound
  (Components|Activation|SetActive (Variables|Default|GetShootSound) false false)
  ;[1 1 1] Stop MuzleFlash
  (Components|Activation|SetActive (Variables|Default|GetMuzzleFlash) false false)
  ;[1 1 1] Stop Camera Shake
  (CameraShake|StopAllCameraShakes (Variables|Default|GetCameraShakeSource) false))

(event Custom|Startfx
  (bind _owningcharacter (Variables|Default|GetOwningCharacter))
  ;[1 1 1] Play Shoot Animation
  (Utilities|IsValid _owningcharacter
    (:Is%20Valid
      (Animation|Montage|PlayMontage (Variables|/Game/UE_FPS/Core/BP_ShooterCharacter.BP_ShooterCharacter_C|GetMesh1P _owningcharacter) (Variables|Default|GetFireMontage)
        (:then
          _)))
    (:Is%20Not%20Valid
      _))
  ;[1 1 1] Play Sound
  (Components|Activation|SetActive (Variables|Default|GetShootSound) true false)
  ;[1 1 1] Show MuzzleFlash
  (Components|Activation|SetActive (Variables|Default|GetMuzzleFlash) true false)
  ;[1 1 1] Play Camera Shake
  (CameraShake|Start (Variables|Default|GetCameraShakeSource)))

(event EventStartFire
  (|CallParentFunction)
  ;[1 1 1] Only Fire Once Until Reset
  (Utilities|FlowControl|DoOnce false :!label _label
    (:Completed
      ;[1 1 1] Play Sound,Muzzle Flash,Animations
      (CallFunction|Startfx)
      ;[1 1 1] Spawn a Projectile
      (Game|SpawnActorfromClass "/Game/UE_FPS/Core/BP_ProjectTile_Grenade.BP_ProjectTile_Grenade_C" (Transformation|GetWorldTransform (Variables|Default|GetMuzzleArrow)) "Undefined" 0 (Variables|Default|GetInstigator))
      ;[1 1 1] Wait a bit Befor allowing to fire another grenade
      (Utilities|FlowControl|Delay (Variables|Default|GetFire%20Time))
      (goto _label Reset))))

(event EventStopFire
  (|CallParentFunction)
  (CallFunction|Stopfx))

(fn ConstructionScript
  (|CallParentFunction)
  (Variables|Default|SetType "NewEnumerator1")
  (Variables|Default|SetFireMontage "/Game/Animations/FPP_Animations/HeroFPP_LauncherFire_Montage.HeroFPP_LauncherFire_Montage")
  (Audio|Components|Audio|SetSound (Variables|Default|GetShootSound) "/Game/Sounds/Weapons/GrenadeLauncher/SCue_Launcher_Shoot.SCue_Launcher_Shoot")
  (Effects|Components|ParticleSystem|SetTemplate (Variables|Default|GetMuzzleFlash) "/Game/Effects/ParticleSystems/Weapons/RocketLauncher/Muzzle/P_Launcher_MF.P_Launcher_MF")
  (Variables|/Script/Engine.CameraShakeSourceComponent|SetCameraShake (Variables|Default|GetCameraShakeSource) "/Game/UE_FPS/Core/WeapLauncher_FireCameraShake.WeapLauncher_FireCameraShake_C"))