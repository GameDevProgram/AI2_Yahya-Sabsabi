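; Rifle weapon Blueprint that adds automatic hitscan fire to its parent weapon's start and stop fire events.
; A looping FireRate timer calls FireBullet, which runs ten identical line traces from the muzzle, applying point damage on hits.
; The trace end multiplies camera location by the forward offset instead of adding, as an in-graph comment flags.
; Montage, looping sound, muzzle flash and camera shake start with firing; stopping adds a tail sound, then ends them.
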(event Custom|Stopfx
  (bind _owningcharacter (Variables|Default|GetOwningCharacter))
  ;[1 1 1] Stop Fire Animation Montage
  (Utilities|IsValid _owningcharacter
    (:Is%20Valid
      (Animation|Montage|MontageStop (Components|SkeletalMesh|GetAnimInstance (Variables|/Game/UE_FPS/Core/BP_ShooterCharacter.BP_ShooterCharacter_C|GetMesh1P _owningcharacter)) 0.1 "/Game/Animations/FPP_Animations/HerroFPP_RifleFire_Montage.HerroFPP_RifleFire_Montage"))
    (:Is%20Not%20Valid
      _))
  ;[1 1 1] Stop Sound
  (Components|Activation|SetActive (Variables|Default|GetShootSound) false false)
  ;[1 1 1] Stop MuzleFlash
  (Components|Activation|SetActive (Variables|Default|GetMuzzleFlash) false false)
  ;[1 1 1] Stop Camera Shake
  (CameraShake|StopAllCameraShakes (Variables|Default|GetCameraShakeSource) false))

(event Custom|Startfx
  (bind _owningcharacter (Variables|Default|GetOwningCharacter))
  ;[1 1 1] Play Shoot Animation
  (Utilities|IsValid _owningcharacter
    (:Is%20Valid
      (Animation|Montage|PlayMontage (Variables|/Game/UE_FPS/Core/BP_ShooterCharacter.BP_ShooterCharacter_C|GetMesh1P _owningcharacter) (Variables|Default|GetFireMontage)
        (:then
          _)))
    (:Is%20Not%20Valid
      _))
  ;[1 1 1] Play Sound
  (Components|Activation|SetActive (Variables|Default|GetShootSound) true false)
  ;[1 1 1] Show MuzzleFlash
  (Components|Activation|SetActive (Variables|Default|GetMuzzleFlash) true false)
  ;[1 1 1] Play Camera Shake
  (CameraShake|Start (Variables|Default|GetCameraShakeSource)))

(event Custom|FireBullet
  (bind _owningcharacter (Variables|Default|GetOwningCharacter))
  (bind _playercamera (Variables|/Game/UE_FPS/Core/BP_ShooterCharacter.BP_ShooterCharacter_C|GetPlayerCamera _owningcharacter))
  ;[1 1 1] Spawn Bullet
  (for _index (range 0 9)
    (bind (_outhit _returnvalue) (Collision|LineTraceByChannel (Transformation|GetWorldLocation (Variables|Default|GetMuzzleArrow)) (* (Transformation|GetWorldLocation _playercamera) (* (Math|Vector|GetForwardVector _playercamera) (Variables|Default|GetRange))) "TraceTypeQuery1" false (Utilities|Array|MakeArray _owningcharacter) "None"))
    (if _returnvalue
      (Game|Damage|ApplyPointDamage (.HitActor (Collision|BreakHitResult _outhit)) 5.0 (.ImpactNormal (Collision|BreakHitResult _outhit)) _outhit (Pawn|GetController (Variables|Default|GetOwningCharacter)) self))))

(event EventStopFire
  (|CallParentFunction)
  ;[1 1 1] Stop Firing Timer
  (Utilities|Time|ClearandInvalidateTimerbyHandle (Variables|Default|GetFiring%20Timer))
  ;[1 1 1] Play end Shooting Sound
  (Audio|PlaySoundatLocation "/Game/Sounds/Weapons/AssultRifle/SCue_AR_Shoot_LP_Tail.SCue_AR_Shoot_LP_Tail" (Transformation|GetActorLocation) "0, 0, 0" 1.0 1.0 0.0 0 0 0)
  (Utilities|FlowControl|Delay 0.1)
  (CallFunction|Stopfx))

(event EventStartFire
  (|CallParentFunction)
  ;[1 1 1] Setup and Start Firing Timer
  (bind _returnvalue (Utilities|Time|SetTimerbyEvent (delegate Custom|FireBullet) (Math|Float|SafeDivide 1.0 (Variables|Default|GetFire%20Rate)) true))
  (Variables|Default|SetFiring%20Timer _returnvalue)
  (CallFunction|FireBullet)
  (CallFunction|Startfx))

(fn ConstructionScript
  (|CallParentFunction)
  (Audio|Components|Audio|SetSound (Variables|Default|GetShootSound) "/Game/Sounds/Weapons/AssultRifle/SCue_AR_Shoot_LP.SCue_AR_Shoot_LP"))