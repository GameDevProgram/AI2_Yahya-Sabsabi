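; Grenade projectile that explodes shortly after its first hit, dealing radial damage around the impact point.
; The Hit event passes through a DoOnce and a brief delay, then applies damage with falloff, credited to the instigator's controller.
; It then spawns the launcher impact emitter at its own location, plays the impact sound at the world origin and destroys itself.
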(event EventBeginPlay)

(event Collision|EventActorBeginOverlap
  (params (OtherActor :type Actor%20Object%20Reference)))

(event EventTick
  (params (DeltaSeconds :type Float%20%28single-precision%29)))

(event Collision|EventHit
  (params (MyComp :type Primitive%20Component%20Object%20Reference) (Other :type Actor%20Object%20Reference) (OtherComp :type Primitive%20Component%20Object%20Reference) (bSelfMoved :type Boolean) (HitLocation :type Vector :default "0, 0, 0") (HitNormal :type Vector :default "0, 0, 0") (NormalImpulse :type Vector :default "0, 0, 0") (Hit :type Hit%20Result%20Structure%20%28by%20ref%29))
  (Utilities|FlowControl|DoOnce false
    (:Completed
      (Utilities|FlowControl|Delay 0.1)
      ;[1 1 1] Apply Damage
      (Class|GameplayStatics|ApplyRadialDamagewithFalloff (Variables|Default|GetDamage) 2e+01 HitLocation 0.0 (Variables|Default|GetDamage%20Radius) 0.5 0 0 self (Game|GetInstigatorController) "ECC_Visibility")
      ;[1 1 1] Show Explosion with Sound
      (Effects|SpawnEmitteratLocation "/Game/Effects/ParticleSystems/Weapons/RocketLauncher/Impact/P_Launcher_IH.P_Launcher_IH" (Transformation|GetActorLocation))
      (Audio|PlaySoundatLocation "/Game/Sounds/Impacts/SCue_Impt_Launcher.SCue_Impt_Launcher" "0, 0, 0" "0, 0, 0" 1.0 1.0 0.0 0 0 0)
      (Actor|DestroyActor))))

(fn ConstructionScript)